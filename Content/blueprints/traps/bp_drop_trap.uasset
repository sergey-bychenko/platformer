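; A drop trap whose plate shakes and falls away when the third-person character enters its trigger box.
; The overlap saves the plate's transform and runs a Shake timeline that adds random jitter to its rotation.
; Shortly after the shake, physics simulation lets the plate drop.
; After a few seconds it stops simulating, returns to the saved transform and zeroes its rotation to reset.
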(event `self.Box.OnComponentBeginOverlap`
  (params (OverlappedComponent :type "PrimitiveComponent Object Reference") (OtherActor :type "Actor Object Reference") (OtherComp :type "PrimitiveComponent Object Reference") (OtherBodyIndex :type Integer) (bFromSweep :type Boolean) (SweepResult :type "HitResult Structure (by ref)"))
  (bind _plate (`self.plate`))
  (bind _plate_2 (`self.plate`))
  (bind (_returnvalue_roll _returnvalue_pitch _returnvalue_yaw) (`KismetMathLibrary.BreakRotator` (`SceneComponent.K2_GetComponentRotation` _plate)))
  (cast `/Game/ThirdPerson/Blueprints/BP_ThirdPersonCharacter` OtherActor)
  (set `self.save_transform` (`SceneComponent.K2_GetComponentToWorld` _plate))
  (bind (_direction _newtrack_0) (`Timeline|shake`)
    (:`Update`
      (bind _returnvalue (* _newtrack_0 (`KismetMathLibrary.RandomFloatInRange` -3.0 3.0)))
      (`SceneComponent.K2_SetWorldRotation` _plate (`KismetMathLibrary.MakeRotator` (+ _returnvalue _returnvalue_roll) (+ _returnvalue _returnvalue_pitch) (+ _returnvalue _returnvalue_yaw)) false false))
    (:`Finished`
      (`KismetSystemLibrary.Delay` 0.5)
      (`PrimitiveComponent.SetSimulatePhysics` _plate true)
      (`KismetSystemLibrary.Delay` 5.0)
      (`PrimitiveComponent.SetSimulatePhysics` _plate false)
      (`SceneComponent.K2_SetWorldTransform` _plate_2 (`self.save_transform`) false false)
      (`TimelineComponent.SetNewTime` (`self.shake`) 0.0)
      (`SceneComponent.K2_SetWorldRotation` _plate_2 (`KismetMathLibrary.MakeRotator` 0.0) false false))))

(fn `UserConstructionScript`)