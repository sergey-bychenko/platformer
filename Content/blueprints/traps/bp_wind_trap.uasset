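; Wind trap actor that pushes the player character around while they stand inside its Wind_box volume.
; A two-second loop from BeginPlay randomizes the X and Y of WindDirection.
; Tick applies the normalized direction times Power as a CharacterMovement force while IsOnBox is set.
; Entering the box zeroes ground friction and overrides braking friction, and leaving writes back hardcoded friction values.
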(event `self.ReceiveBeginPlay`
  (`KismetSystemLibrary.Delay` 2.0 :!label _label)
  (`KismetMathLibrary.Vector_Set` (`self.wind_direction`) (`KismetMathLibrary.RandomFloatInRange` -1.0 1.0) (`KismetMathLibrary.RandomFloatInRange` -1.0 1.0))
  (goto _label))

(event `self.ReceiveActorBeginOverlap`
  (params (OtherActor :type "Actor Object Reference")))

(event `self.ReceiveTick`
  (params (DeltaSeconds :type "Float (single-precision)"))
  (if (`self.is_on_box`)
    (bind _asbp_third_person_character (cast `/Game/ThirdPerson/Blueprints/BP_ThirdPersonCharacter` (`GameplayStatics.GetPlayerCharacter` 0)))
    (`CharacterMovementComponent.AddForce` (`Character.CharacterMovement` _asbp_third_person_character) (* (`KismetMathLibrary.Normal` (`self.wind_direction`)) (`self.power`)))))

(event `self.wind_box.OnComponentBeginOverlap`
  (params (OverlappedComponent :type "PrimitiveComponent Object Reference") (OtherActor :type "Actor Object Reference") (OtherComp :type "PrimitiveComponent Object Reference") (OtherBodyIndex :type Integer) (bFromSweep :type Boolean) (SweepResult :type "HitResult Structure (by ref)"))
  (bind _asbp_third_person_character (cast `/Game/ThirdPerson/Blueprints/BP_ThirdPersonCharacter` OtherActor))
  (set `self.is_on_box` true)
  (bind _charactermovement (`Character.CharacterMovement` _asbp_third_person_character))
  (set `CharacterMovementComponent.GroundFriction` 0.0 _charactermovement)
  (set `CharacterMovementComponent.BrakingFriction` (`self.brkn_frctn`) _charactermovement))

(event `self.wind_box.OnComponentEndOverlap`
  (params (OverlappedComponent :type "PrimitiveComponent Object Reference") (OtherActor :type "Actor Object Reference") (OtherComp :type "PrimitiveComponent Object Reference") (OtherBodyIndex :type Integer))
  (cast `/Game/ThirdPerson/Blueprints/BP_ThirdPersonCharacter` OtherActor)
  (set `self.is_on_box` false)
  (bind _charactermovement (`Character.CharacterMovement` (stale `self.wind_box.OnComponentBeginOverlap` _asbp_third_person_character)))
  (set `CharacterMovementComponent.GroundFriction` 8.0 _charactermovement)
  (set `CharacterMovementComponent.BrakingFriction` 2000.0 _charactermovement))

(fn `UserConstructionScript`)