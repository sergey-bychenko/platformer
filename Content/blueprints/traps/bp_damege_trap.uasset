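; BP_Damege_Trap is a floor plate trap that damages the player standing on it.
; Overlap with the third-person character starts a timed cycle: warning material, delayed damage to player 0 if still flagged on the platform, flash, then cooldown.
; The cycle repeats while the occupancy flag holds, and a reloading flag blocks re-triggering.
; Any actor's overlap sets or clears occupancy, because the flag changes outside the character cast.
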(event `self.colision.OnComponentBeginOverlap`
  (params (OverlappedComponent :type "PrimitiveComponent Object Reference") (OtherActor :type "Actor Object Reference") (OtherComp :type "PrimitiveComponent Object Reference") (OtherBodyIndex :type Integer) (bFromSweep :type Boolean) (SweepResult :type "HitResult Structure (by ref)"))
  (bind _plate (`self.plate`))
  (set `self.is_player_on_platform` true)
  (cast `/Game/ThirdPerson/Blueprints/BP_ThirdPersonCharacter` OtherActor)
  (if (not (`self.is_reloading`))
    (set `self.is_reloading` true)
    (`PrimitiveComponent.SetMaterial` _plate 0 "/Engine/TemplateResources/MI_Template_BaseOrange.MI_Template_BaseOrange" :!label _label)
    (`KismetSystemLibrary.Delay` 1.0)
    (if (`self.is_player_on_platform`)
      (`GameplayStatics.ApplyDamage` (`GameplayStatics.GetPlayerCharacter` 0) 20.0))
    (`PrimitiveComponent.SetMaterial` _plate 0 "/Engine/VREditor/LaserPointer/LaserPointerMaterial.LaserPointerMaterial")
    (`KismetSystemLibrary.Delay` 0.5)
    (`PrimitiveComponent.SetMaterial` _plate 0 "/Game/LevelPrototyping/Materials/MI_Solid_Blue.MI_Solid_Blue")
    (`KismetSystemLibrary.Delay` 5.0)
    (if (`self.is_player_on_platform`)
      (goto _label)
      (else
        (set `self.is_reloading` false)))))

(event `self.colision.OnComponentEndOverlap`
  (params (OverlappedComponent :type "PrimitiveComponent Object Reference") (OtherActor :type "Actor Object Reference") (OtherComp :type "PrimitiveComponent Object Reference") (OtherBodyIndex :type Integer))
  (set `self.is_player_on_platform` false))

(fn `UserConstructionScript`)