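; Checkpoint trigger actor that serves as either the start or the finish of a timed run, selected by the IsFinsihCheckpoint flag.
; When a BP_ThirdPersonCharacter begins overlapping its Box, it casts player controller 0 to bp_person_ui, which handles the timer.
; A start checkpoint calls StartTimer, while a finish checkpoint calls PauseTimer and then FinishGame, with debug prints on both paths.
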(event `self.Box.OnComponentBeginOverlap`
  (params (OverlappedComponent :type "PrimitiveComponent Object Reference") (OtherActor :type "Actor Object Reference") (OtherComp :type "PrimitiveComponent Object Reference") (OtherBodyIndex :type Integer) (bFromSweep :type Boolean) (SweepResult :type "HitResult Structure (by ref)"))
  (bind _returnvalue (`GameplayStatics.GetPlayerController` 0))
  (cast `/Game/ThirdPerson/Blueprints/BP_ThirdPersonCharacter` OtherActor)
  (if (`self.is_finsih_checkpoint`)
    (bind _asbp_person_ui (cast `/Game/blueprints/bp_person_ui` _returnvalue))
    (`/Game/blueprints/bp_person_ui.pause_timer` _asbp_person_ui)
    (`KismetSystemLibrary.PrintString` "pause")
    (bind _asbp_person_ui_2 (cast `/Game/blueprints/bp_person_ui` (`GameplayStatics.GetPlayerController` 0)))
    (`/Game/blueprints/bp_person_ui.finish_game` _asbp_person_ui_2 true)
    (else
      (bind _asbp_person_ui_3 (cast `/Game/blueprints/bp_person_ui` _returnvalue))
      (`/Game/blueprints/bp_person_ui.start_timer` _asbp_person_ui_3)
      (`KismetSystemLibrary.PrintString` "start"))))

(fn `UserConstructionScript`)